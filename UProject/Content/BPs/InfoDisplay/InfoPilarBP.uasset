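; Info pillar actor whose info display rotates in response to VR headset orientation.
; Entering or leaving the trigger sphere toggles visibility and stores the current HMD rotation as a reference.
; While the display is visible, Tick adds a scaled-down offset from that reference as relative rotation, with yaw and roll swapped.
; The offset accumulates each frame, so head angle sets spin speed rather than absolute orientation.
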(event `self.TriggerSphere.OnComponentBeginOverlap`
  (params (OtherActor :type "Actor Object Reference") (OtherComp :type "PrimitiveComponent Object Reference") (OtherBodyIndex :type Integer) (bFromSweep :type Boolean) (SweepResult :type "EngineTypes.HitResult Structure (by ref)"))
  (`SceneComponent.ToggleVisibility` false :!label _label)
  (set `self.CurrentRotation` (`HeadMountedDisplayFunctionLibrary.GetOrientationAndPosition`)))

(event `self.TriggerSphere.OnComponentEndOverlap`
  (params (OtherActor :type "Actor Object Reference") (OtherComp :type "PrimitiveComponent Object Reference") (OtherBodyIndex :type Integer))
  (goto _label))

(event `self.ReceiveTick`
  (params (DeltaSeconds :type "Float (single-precision)"))
  (if (`SceneComponent.bVisible` (`self.infoDisplay`))
    (`SceneComponent.K2_AddRelativeRotation` (`self.infoDisplay`) (`KismetMathLibrary.MakeRot` (.pitch (* (`KismetMathLibrary.NormalizedDeltaRotator` (`HeadMountedDisplayFunctionLibrary.GetOrientationAndPosition`) (`self.CurrentRotation`)) 0.1)) (.roll (* (`KismetMathLibrary.NormalizedDeltaRotator` (`HeadMountedDisplayFunctionLibrary.GetOrientationAndPosition`) (`self.CurrentRotation`)) 0.1)) (.yaw (* (`KismetMathLibrary.NormalizedDeltaRotator` (`HeadMountedDisplayFunctionLibrary.GetOrientationAndPosition`) (`self.CurrentRotation`)) 0.1))) true)))

(fn `UserConstructionScript`)