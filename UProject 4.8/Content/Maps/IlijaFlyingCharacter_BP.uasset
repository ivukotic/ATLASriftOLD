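; VR flying character that lets the player navigate head-controlled menus for a detector tour, subdetector options and events.
; A Level state machine advances on MainMenu presses, while Tick moves the active menu from headset rotation relative to a captured baseline, with a jitter threshold.
; Menu rotation or cursor offset picks options: a timeline-driven narrated tour, or hiding and showing tag-matched actors.
; Other manipulation options only print; backMenu resets everything.
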(event `InputAxis|MoveUp`
  (params (AxisValue :type "Float (single-precision)"))
  (`self.K2_SetActorLocation` (+ (`KismetMathLibrary.MakeVector` 0.0 0.0 AxisValue) (`self.K2_GetActorLocation`))))

(event `InputAction|MainMenu`
  (bind _eventcounter (`self.eventCounter`))
  (bind (_remainder _returnvalue) (`KismetMathLibrary.FMod` (+ 190.588235 (.yaw (`SceneComponent.RelativeRotation` (`self.submenu-detector`)))) 21.17647))
  (bind (_remainder_2 _returnvalue_2) (`KismetMathLibrary.FMod` (+ 225.0 (.yaw (`SceneComponent.RelativeRotation` (`self.MM`)))) 90.0))
  (bind (_remainder_3 _returnvalue_3) (`KismetMathLibrary.FMod` (+ 190.588235 (.yaw (`SceneComponent.RelativeRotation` (`self.submenu-detector`)))) 21.17647))
  (bind (_remainder_4 _returnvalue_4) (`KismetMathLibrary.FMod` (+ 62.0 (.z (`SceneComponent.RelativeLocation` (`SceneComponent.GetChildComponent` (`SceneComponent.GetChildComponent` (`self.subdetmanip`) 0) 2)))) 25.0))
  (:`Pressed`
    (switch `int` (`self.level`)
      (:`0`
        (set `self.level` 1)
        (`self.Enable Main Menu`))
      (:`1`
        (set `self.level` 2)
        (`KismetSystemLibrary.PrintString` (`KismetStringLibrary.Conv_IntToString` _returnvalue_2) false)
        ;[1 1 1] 0|4- tour 1-detector 2-event 3 - about
        (switch `int` _returnvalue_2
          (:`0`
            (`self.AllReset` :!label _label)
            (`AudioComponent.Play` (`self.GuideVoiceComponent`) 0.0)
            (bind (_direction _locationtrack) (`Timeline|TourTimeline` :!via `PlayFromStart` :!label _label_2)
              (:`Update`
                (`self.K2_SetActorLocation` (`GameplayStatics.GetPlayerPawn` 0) _locationtrack false))
              (:`EventsAlongTrack`
                (`self.TimeLineDispatch` _eventcounter)
                (set `self.eventCounter` (+ _eventcounter 1)))))
          (:`1`
            (`self.Enable Detector SubMenu`))
          (:`2`
            (`self.AllReset`)
            (set `self.level` 4)
            (`self.Enable Event Sub Menu`))
          (:`3`
            (`self.AllReset`))
          (:`4`
            (goto _label))))
      (:`2`
        (set `self.level` 3)
        (set `self.selectedOption` _returnvalue)
        (`KismetSystemLibrary.PrintString` (`KismetStringLibrary.Conv_IntToString` _returnvalue) false)
        (`self.Enable SubDetectorManipulation`))
      (:`3`
        (`KismetSystemLibrary.PrintString` (`KismetStringLibrary.Conv_IntToString` _returnvalue_4) false false)
        (bind _outactors (`GameplayStatics.GetAllActorsOfClass` "/Script/Engine.Actor"))
        (for _array_element _outactors
          (bind _tags (`Actor.Tags` _array_element))
          (if (> (`KismetArrayLibrary.Array_Length` _tags) 0)
            (if (== (`KismetArrayLibrary.Array_Get` _tags) (`KismetStringLibrary.Conv_StringToName` (`KismetStringLibrary.Conv_IntToString` (`self.selectedOption`))))
              (`KismetSystemLibrary.PrintString` "found actor" false)
              (`KismetSystemLibrary.PrintString` (`KismetSystemLibrary.GetDisplayName` _array_element) false)
              (switch `int` _returnvalue_4
                (:`0`
                  (`KismetSystemLibrary.PrintString` "Tour"))
                (:`1`
                  (`KismetSystemLibrary.PrintString` "Gallery"))
                (:`2`
                  (`KismetSystemLibrary.PrintString` "Visible")
                  (`self.SetActorHiddenInGame` _array_element false))
                (:`3`
                  (`KismetSystemLibrary.PrintString` "Invisible")
                  (`self.SetActorHiddenInGame` _array_element true))
                (:`4`
                  (`KismetSystemLibrary.PrintString` "Translcent")))))))
      (:`4`
        (set `self.level` 5)
        (set `self.selectedOption` _returnvalue_3)
        (`KismetSystemLibrary.PrintString` (`KismetStringLibrary.Conv_IntToString` _returnvalue_3) false)
        (`self.AllReset`)))))

(event `InputAction|backMenu`
  (:`Pressed`
    (`self.AllReset`)
    (`KismetSystemLibrary.PrintString` "Full menu reset" false)
    (`AudioComponent.Stop` (`self.GuideVoiceComponent`))
    (goto _label_2 :!via `Stop`)))

(event `self.ReceiveTick`
  (params (DeltaSeconds :type "Float (single-precision)"))
  (switch `int` (`self.level`)
    (:`1`
      (`self.RunMainMenu`))
    (:`2`
      (`self.Run Detector SubMenu`))
    (:`3`
      (`self.Run Sub Detector Manipulation`))
    (:`4`
      (`self.Run Event Sub Menu`))))

(fn `AllReset`
  (set `self.level` 0)
  (set `self.selectedOption` 0)
  (`SceneComponent.SetVisibility` false true)
  (`SceneComponent.SetVisibility` false true)
  (`SceneComponent.SetVisibility` false true)
  (`SceneComponent.SetVisibility` false true)
  (`SceneComponent.SetVisibility` (`self.HeadLamp`) false false))

(fn `Enable Detector SubMenu`
  (`SceneComponent.SetVisibility` (`self.MM`) false false)
  (`SceneComponent.SetVisibility` true true)
  (set `self.BaseRotation` (`HeadMountedDisplayFunctionLibrary.GetOrientationAndPosition`))
  (`GameplayStatics.PlaySoundAtLocation` "/Game/Audio/Woosh-Mark_DiAngelo-4778593.Woosh-Mark_DiAngelo-4778593" (`self.K2_GetActorLocation`))
  (`KismetSystemLibrary.PrintString` "Activated Detector Sub Menu" false))

(fn `Enable Event Sub Menu`
  (`SceneComponent.SetVisibility` true true)
  (set `self.BaseRotation` (`HeadMountedDisplayFunctionLibrary.GetOrientationAndPosition`))
  (`GameplayStatics.PlaySoundAtLocation` "/Game/Audio/Woosh-Mark_DiAngelo-4778593.Woosh-Mark_DiAngelo-4778593" (`self.K2_GetActorLocation`))
  (`KismetSystemLibrary.PrintString` "Activated Sub Menu Event" false))

(fn `Enable Main Menu`
  (`SceneComponent.SetVisibility` (`self.MM`) true false)
  (`SceneComponent.SetVisibility` (`self.HeadLamp`) true false)
  (set `self.BaseRotation` (`HeadMountedDisplayFunctionLibrary.GetOrientationAndPosition`))
  (`GameplayStatics.PlaySoundAtLocation` "/Game/Audio/Woosh-Mark_DiAngelo-4778593.Woosh-Mark_DiAngelo-4778593" (`self.K2_GetActorLocation`))
  (`KismetSystemLibrary.PrintString` "Activated Main Menu" false))

(fn `Enable SubDetectorManipulation`
  (`SceneComponent.SetVisibility` false true)
  (`SceneComponent.SetVisibility` true true)
  (set `self.BaseRotation` (`HeadMountedDisplayFunctionLibrary.GetOrientationAndPosition`))
  (`GameplayStatics.PlaySoundAtLocation` "/Game/Audio/Woosh-Mark_DiAngelo-4778593.Woosh-Mark_DiAngelo-4778593" (`self.K2_GetActorLocation`))
  (`KismetSystemLibrary.PrintString` "Activated Sub Detector Manipulation" false))

(fn `Run Detector SubMenu`
  (bind _yaw (.yaw (* (`KismetMathLibrary.NormalizedDeltaRotator` (`HeadMountedDisplayFunctionLibrary.GetOrientationAndPosition`) (`self.BaseRotation`)) 0.1)))
  (if (`SceneComponent.bVisible` (`self.submenu-detector`))
    (if (> (`KismetMathLibrary.Abs` _yaw) 0.1)
      (`SceneComponent.K2_AddLocalRotation` (`self.submenu-detector`) (`KismetMathLibrary.MakeRot` 0.0 _yaw) false))))

(fn `Run Event Sub Menu`
  (bind _pitch (.pitch (* (`KismetMathLibrary.NormalizedDeltaRotator` (`HeadMountedDisplayFunctionLibrary.GetOrientationAndPosition`) (`self.BaseRotation`)) 3.0)))
  (bind _yaw (.yaw (* (`KismetMathLibrary.NormalizedDeltaRotator` (`HeadMountedDisplayFunctionLibrary.GetOrientationAndPosition`) (`self.BaseRotation`)) 3.0)))
  ;[1 1 1] unneeded
  (if (`SceneComponent.bVisible` (`self.submenu-event`))
    (if (or (> (`KismetMathLibrary.Abs` _pitch) 0.1) (> (`KismetMathLibrary.Abs` _yaw) 0.1))
      (`SceneComponent.K2_SetRelativeLocation` (`SceneComponent.GetChildComponent` (`SceneComponent.GetChildComponent` (`self.submenu-event`) 0) 1) (`KismetMathLibrary.MakeVector` 0.0 _yaw _pitch) false))))

(fn `Run Sub Detector Manipulation`
  (bind _pitch (.pitch (* (`KismetMathLibrary.NormalizedDeltaRotator` (`HeadMountedDisplayFunctionLibrary.GetOrientationAndPosition`) (`self.BaseRotation`)) 2.0)))
  ;[1 1 1] unneeded
  (if (`SceneComponent.bVisible` (`self.subdetmanip`))
    (if (> (`KismetMathLibrary.Abs` _pitch) 0.1)
      (`SceneComponent.K2_SetRelativeLocation` (`SceneComponent.GetChildComponent` (`SceneComponent.GetChildComponent` (`self.subdetmanip`) 0) 2) (`KismetMathLibrary.MakeVector` 0.0 0.0 _pitch) false))))

(fn `RunMainMenu`
  (bind _yaw (.yaw (* (`KismetMathLibrary.NormalizedDeltaRotator` (`HeadMountedDisplayFunctionLibrary.GetOrientationAndPosition`) (`self.BaseRotation`)) 0.1)))
  (if (`SceneComponent.bVisible` (`self.MM`))
    (if (> (`KismetMathLibrary.Abs` _yaw) 0.1)
      (`SceneComponent.K2_AddRelativeRotation` (`self.MM`) (`KismetMathLibrary.MakeRot` 0.0 _yaw) false))))

(fn `UserConstructionScript`)