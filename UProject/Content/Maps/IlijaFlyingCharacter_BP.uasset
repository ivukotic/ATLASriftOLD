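; VR flying character with head-steered menus for a guided tour, detector submenu and event submenu.
; MainMenu input advances a Level state machine and backMenu resets it, while Tick runs the active level's handler.
; Headset rotation relative to a captured baseline, with a jitter deadzone, spins menus or slides child components.
; Menu yaw divided into sectors picks the option; Tour plays a timeline moving the pawn with guide audio.
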(event `InputAction|backMenu`
  (:`Pressed`
    (`self.AllReset`)))

(event `InputAction|MainMenu`
  (bind (_remainder _returnvalue) (`KismetMathLibrary.FMod` (+ 225.0 (.yaw (`SceneComponent.RelativeRotation` (`self.MM`)))) 90.0))
  (bind (_remainder_2 _returnvalue_2) (`KismetMathLibrary.FMod` (+ 190.588235 (.yaw (`SceneComponent.RelativeRotation` (`self.submenu-detector`)))) 21.17647))
  (:`Pressed`
    (switch `int` (`self.level`)
      (:`0`
        (set `self.level` 1)
        (`self.Enable Main Menu`))
      (:`1`
        (set `self.level` 2)
        (`KismetSystemLibrary.PrintString` (`KismetStringLibrary.Conv_IntToString` _returnvalue) false)
        ;[1 1 1] 0|4- tour 1-detector 2-event 3 - about
        (switch `int` _returnvalue
          (:`0`
            (`self.AllReset` :!label _label)
            (bind (_direction _locationtrack) (`Timeline|TourTimeline` :!via `PlayFromStart`)
              (:`Update`
                (`self.K2_SetActorLocation` (`GameplayStatics.GetPlayerPawn` 0) _locationtrack false))
              (:`EventsAlongTrack`
                (`KismetSystemLibrary.PrintString` "PLAYING SOUND" false)
                (`GameplayStatics.PlaySoundAtLocation` "/Game/Audio/MyTourGuide.MyTourGuide" _locationtrack 2.0))))
          (:`1`
            (`self.Enable Detector SubMenu`))
          (:`2`
            (`self.AllReset`)
            (set `self.level` 4)
            (`self.Enable Event Sub Menu`))
          (:`3`
            (`self.AllReset`))
          (:`4`
            (goto _label))))
      (:`2`
        (set `self.level` 3)
        (set `self.selectedOption` _returnvalue_2)
        (`KismetSystemLibrary.PrintString` (`KismetStringLibrary.Conv_IntToString` _returnvalue_2) false)
        (`self.Enable SubDetectorManipulation`)))))

(event `self.ReceiveTick`
  (params (DeltaSeconds :type "Float (single-precision)"))
  (switch `int` (`self.level`)
    (:`1`
      (`self.RunMainMenu`))
    (:`2`
      (`self.Run Detector SubMenu`))
    (:`3`
      (`self.Run Sub Detector Manipulation`))
    (:`4`
      (`self.Run Event Sub Menu`))))

(fn `AllReset`
  (set `self.level` 0)
  (set `self.selectedOption` 0)
  (`SceneComponent.SetVisibility` (`self.submenu-detector`) false true)
  (`SceneComponent.SetVisibility` (`self.MM`) false false)
  (`SceneComponent.SetVisibility` false true))

(fn `Enable Detector SubMenu`
  (`SceneComponent.SetVisibility` (`self.MM`) false false)
  (`SceneComponent.SetVisibility` true true)
  (set `self.BaseRotation` (`HeadMountedDisplayFunctionLibrary.GetOrientationAndPosition`))
  (`GameplayStatics.PlaySoundAtLocation` "/Game/Audio/Woosh-Mark_DiAngelo-4778593.Woosh-Mark_DiAngelo-4778593" (`self.K2_GetActorLocation`))
  (`KismetSystemLibrary.PrintString` "Activated Detector Sub Menu" false))

(fn `Enable Event Sub Menu`
  (`SceneComponent.SetVisibility` true true)
  (set `self.BaseRotation` (`HeadMountedDisplayFunctionLibrary.GetOrientationAndPosition`))
  (`GameplayStatics.PlaySoundAtLocation` "/Game/Audio/Woosh-Mark_DiAngelo-4778593.Woosh-Mark_DiAngelo-4778593" (`self.K2_GetActorLocation`))
  (`KismetSystemLibrary.PrintString` "Activated Sub Menu Event" false))

(fn `Enable Main Menu`
  (`SceneComponent.SetVisibility` (`self.MM`) true false)
  (set `self.BaseRotation` (`HeadMountedDisplayFunctionLibrary.GetOrientationAndPosition`))
  (`GameplayStatics.PlaySoundAtLocation` "/Game/Audio/Woosh-Mark_DiAngelo-4778593.Woosh-Mark_DiAngelo-4778593" (`self.K2_GetActorLocation`))
  (`KismetSystemLibrary.PrintString` "Activated Main Menu" false))

(fn `Enable SubDetectorManipulation`
  (`SceneComponent.SetVisibility` false true)
  (`SceneComponent.SetVisibility` true true)
  (set `self.BaseRotation` (`HeadMountedDisplayFunctionLibrary.GetOrientationAndPosition`))
  (`GameplayStatics.PlaySoundAtLocation` "/Game/Audio/Woosh-Mark_DiAngelo-4778593.Woosh-Mark_DiAngelo-4778593" (`self.K2_GetActorLocation`))
  (`KismetSystemLibrary.PrintString` "Activated Sub Detector Manipulation" false)
  (for (_array_element _array_index) (`SceneComponent.GetChildrenComponents` (`SceneComponent.GetChildComponent` (`self.subdetmanip`) 0) false)
    (`KismetSystemLibrary.PrintString` (`KismetSystemLibrary.GetDisplayName` _array_element))
    (`KismetSystemLibrary.PrintString` (`KismetStringLibrary.Conv_IntToString` _array_index))))

(fn `Run Detector SubMenu`
  (bind _yaw (.yaw (* (`KismetMathLibrary.NormalizedDeltaRotator` (`HeadMountedDisplayFunctionLibrary.GetOrientationAndPosition`) (`self.BaseRotation`)) 0.1)))
  (if (`SceneComponent.bVisible` (`self.submenu-detector`))
    (if (> (`KismetMathLibrary.Abs` _yaw) 0.1)
      (`SceneComponent.K2_AddLocalRotation` (`self.submenu-detector`) (`KismetMathLibrary.MakeRot` 0.0 _yaw) false))))

(fn `Run Event Sub Menu`
  (bind _pitch (.pitch (* (`KismetMathLibrary.NormalizedDeltaRotator` (`HeadMountedDisplayFunctionLibrary.GetOrientationAndPosition`) (`self.BaseRotation`)) 3.0)))
  (bind _yaw (.yaw (* (`KismetMathLibrary.NormalizedDeltaRotator` (`HeadMountedDisplayFunctionLibrary.GetOrientationAndPosition`) (`self.BaseRotation`)) 3.0)))
  ;[1 1 1] unneeded
  (if (`SceneComponent.bVisible` (`self.submenu-event`))
    (if (or (> (`KismetMathLibrary.Abs` _pitch) 0.1) (> (`KismetMathLibrary.Abs` _yaw) 0.1))
      (`SceneComponent.K2_SetRelativeLocation` (`SceneComponent.GetChildComponent` (`SceneComponent.GetChildComponent` (`self.submenu-event`) 0) 1) (`KismetMathLibrary.MakeVector` 0.0 _yaw _pitch) false))))

(fn `Run Sub Detector Manipulation`
  (bind _pitch (.pitch (* (`KismetMathLibrary.NormalizedDeltaRotator` (`HeadMountedDisplayFunctionLibrary.GetOrientationAndPosition`) (`self.BaseRotation`)) 2.0)))
  ;[1 1 1] unneeded
  (if (`SceneComponent.bVisible` (`self.subdetmanip`))
    (if (> (`KismetMathLibrary.Abs` _pitch) 0.1)
      (`SceneComponent.K2_SetRelativeLocation` (`SceneComponent.GetChildComponent` (`SceneComponent.GetChildComponent` (`self.subdetmanip`) 0) 2) (`KismetMathLibrary.MakeVector` 0.0 0.0 _pitch) false))))

(fn `RunMainMenu`
  (bind _yaw (.yaw (* (`KismetMathLibrary.NormalizedDeltaRotator` (`HeadMountedDisplayFunctionLibrary.GetOrientationAndPosition`) (`self.BaseRotation`)) 0.1)))
  (if (`SceneComponent.bVisible` (`self.MM`))
    (if (> (`KismetMathLibrary.Abs` _yaw) 0.1)
      (`SceneComponent.K2_AddRelativeRotation` (`self.MM`) (`KismetMathLibrary.MakeRot` 0.0 _yaw) false))))

(fn `UserConstructionScript`)